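; Interaction_Master is an interactable actor for click-to-move top-down play that reacts when clicked.
; Clicking briefly disables the top-down controller's input for one tick.
; If the player character is over 200 units away, it moves toward a point just beside the actor; otherwise Interact runs.
; Interact adds one hardcoded MCFish item to the player character through AddItem.
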(event `self.ReceiveBeginPlay`
  (add `self.OnClicked` (delegate `OnClicked_Event`))
  (bind _asbp_top_down_controller (cast `/Game/TopDown/Blueprints/BP_TopDownController` (`GameplayStatics.GetPlayerController` 0)))
  (set `self.As BP Top Down Controller` _asbp_top_down_controller))

(event `OnClicked_Event` :!signature `self.OnClicked`
  (params (TouchedActor :type "Actor Object Reference") (ButtonPressed :type "Key Structure" :default "None"))
  (bind _returnvalue (`self.K2_GetActorLocation`))
  (bind _as_bp_top_down_controller (`self.As BP Top Down Controller`))
  (bind _returnvalue_2 (`self.K2_GetActorLocation` (`GameplayStatics.GetPlayerCharacter` 0)))
  (`self.DisableInput` _as_bp_top_down_controller _as_bp_top_down_controller)
  (`KismetSystemLibrary.DelayUntilNextTick`)
  (`self.EnableInput` _as_bp_top_down_controller _as_bp_top_down_controller)
  (if (> (`KismetMathLibrary.Vector_Distance` _returnvalue _returnvalue_2) 200.0)
    (`AIBlueprintHelperLibrary.SimpleMoveToLocation` (`self.As BP Top Down Controller`) (+ _returnvalue (* (`KismetMathLibrary.GetDirectionUnitVector` _returnvalue _returnvalue_2) 25.0)))
    (else
      (`self.Interact`))))

(event `Interact`
  (`/Game/TopDown/Blueprints/BP_TopDownCharacter.Add Item` (cast `/Game/TopDown/Blueprints/BP_TopDownCharacter` (`GameplayStatics.GetPlayerCharacter` 0) :!pure true) "MCFish" 1))

(fn `UserConstructionScript`)